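; Tadpole actor that travels along a spline path once play begins.
; On BeginPlay it finds all BP_SplinePath actors and uses the first one's spline.
; A timeline, with play rate set from TimeToCompleteInSec, lerps distance over the spline's length to drive the actor's world location and rotation.
; A random-number write to the MPC_Fish parameter collection is present but disconnected, and the Speed variable is unused.
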(event Custom|moveObject
  (bind _spline_ref (Variables|Actor|GetSpline%20REF))
  (bind _output (Utilities|Array|Get(acopy) _spline_ref))
  (bind _spline (Variables|/Game/BP/oldSplineTadpole/BP_SplinePath.BP_SplinePath_C|GetSpline _output))
  (Components|Timeline|SetPlayRate (Variables|Default|GetMove%20Object%20Timeline) (/ 1.0 (Variables|Default|GetTime%20To%20Complete%28In%20Sec%29)))
  (bind _move_track (Timeline|Move%20Object%20Timeline Play)
    (:Update
      (Transformation|SetActorTransform (Math|Transform|MakeTransform (Spline|GetLocationatDistanceAlongSpline _spline (Math|Float|Lerp 0.0 (Spline|GetSplineLength _spline) _move_track) "World") (Spline|GetRotationatDistanceAlongSpline _spline (Math|Float|Lerp 0.0 (Spline|GetSplineLength _spline) _move_track) "World") "1,1,1")))))

(event EventBeginPlay
  (bind _outactors (Actor|GetAllActorsOfClass "/Game/BP/oldSplineTadpole/BP_SplinePath.BP_SplinePath_C"))
  (Variables|Actor|SetSpline%20REF _outactors)
  (CallFunction|MoveObject))

(event EventTick
  (params (DeltaSeconds :type Float%20%28single-precision%29)))

(fn ConstructionScript)